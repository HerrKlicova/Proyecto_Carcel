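; Blueprint function library providing a cone trace that approximates a cone with a flat fan of line traces on the Visibility channel.
; It rotates the forward vector around the cone normal in even steps up to the given angle, testing both sides from the center outward.
; The first blocking hit returns immediately with its hit result, otherwise it returns false, and each trace draws one-frame debug lines.
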(fn `Cone Trace by Channel`
  (params (StartLocation :type "Vector Structure") (NumberOfLines :type Integer) (Angle :type "Float (double-precision)") (ConeLength :type "Float (single-precision)") (ConeForward :type "Vector Structure") (ConeNormal :type "Vector Structure"))
  (returns (OutHit :type "HitResult Structure") (ReturnValue :type Boolean))
  (locals (IncrementAngle :type "Float (double-precision)") (EndLocation :type "Vector Structure") (HitObject :type "HitResult Structure"))
  (bind _numberoflines (`local.NumberOfLines`))
  (bind _conelength (`local.ConeLength`))
  (bind _endlocation (`local.EndLocation`))
  (bind _conenormal (`local.ConeNormal`))
  (bind _coneforward (`local.ConeForward`))
  (bind _startlocation (`local.StartLocation`))
  (bind _incrementangle (`local.IncrementAngle`))
  (for _index (range (+ _numberoflines 1))
    (set `local.IncrementAngle` (* (/ (`local.Angle`) _numberoflines) _index))
    (set `local.EndLocation` (+ _startlocation (* (`KismetMathLibrary.RotateAngleAxis` _coneforward _incrementangle _conenormal) _conelength)))
    (bind (_outhit _returnvalue) (`KismetSystemLibrary.LineTraceSingle` :`Start` _startlocation :`End` _endlocation :`TraceChannel` "TraceTypeQuery1" :`DrawDebugType` "ForOneFrame"))
    (set `local.HitObject` _outhit)
    (if _returnvalue
      (return (`local.HitObject`) true)
      (else
        (set `local.EndLocation` (+ _startlocation (* (`KismetMathLibrary.RotateAngleAxis` _coneforward (* _incrementangle -1.0) _conenormal) _conelength)))
        (bind (_outhit_2 _returnvalue_2) (`KismetSystemLibrary.LineTraceSingle` :`Start` _startlocation :`End` _endlocation :`TraceChannel` "TraceTypeQuery1" :`DrawDebugType` "ForOneFrame"))
        (set `local.HitObject` _outhit_2)
        (if _returnvalue_2
          (return (`local.HitObject`) true)))))
  (return (struct) false))