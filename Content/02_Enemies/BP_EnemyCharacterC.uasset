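; Enemy character that checks whether it can see its target actor and shows the result through the color of its exclamation indicator.
; Each tick, a squared-distance check against the vision radius gates a forward-facing multi-line cone trace.
; A hit on the target turns the indicator green and any other hit red; otherwise the color stays unchanged.
; The construction script starts it blue via a material vector parameter on the Cube.
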(event `self.K2_OnBecomeViewTarget`
  (params (PC :type "PlayerController Object Reference")))

(event `self.K2_OnReset`)

(event `self.ReceiveTick`
  (params (DeltaSeconds :type "Float (single-precision)"))
  (if (<= (`KismetMathLibrary.Vector_DistanceSquared` (`self.K2_GetActorLocation` (`self.TargetActor`)) (`self.K2_GetActorLocation` self)) (`KismetMathLibrary.Square` (`self.VisionRadius`)))
    (bind (_outhit _returnvalue) (`/Game/EinarFolder/BP_FunctionLibrary.Cone Trace by Channel` (+ (`self.K2_GetActorLocation`) (`self.StartOffset`)) (`self.NumberOfLines`) (`self.MaxAngle`) (`self.VisionRadius`) (`self.GetActorForwardVector`) (`self.GetActorUpVector`)))
    (if _returnvalue
      (if (== (`.HitActor` (`GameplayStatics.BreakHitResult` _outhit)) (`self.TargetActor`))
        (`self.SetExclamationColor` (struct :`R` 0.132907 :`G` 1.0 :`A` 1.0))
        (else
          (`self.SetExclamationColor` (struct :`R` 1.0 :`B` 0.061241 :`A` 1.0)))))))

(fn `SetExclamationColor`
  (params (InLinearColor :type "LinearColor Structure" :default (struct :`R` 1.0 :`B` 0.061241 :`A` 1.0)))
  (`MeshComponent.SetVectorParameterValueOnMaterials` (`self.Cube`) "Color" (`KismetMathLibrary.Conv_LinearColorToVector` InLinearColor)))

(fn `UserConstructionScript`
  (`self.SetExclamationColor` (struct :`G` 0.034317 :`B` 1.0 :`A` 1.0)))